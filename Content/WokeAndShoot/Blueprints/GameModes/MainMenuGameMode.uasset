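; Main menu game mode for WokeAndShoot that exposes HostGame and JoinGame events for starting or joining a multiplayer session.
; Each event calls a helper function that casts the game instance to MyGameInstance and forwards to its HostGameImplem or JoinGameImplem, passing the server IP when joining.
; A failed cast prints a message when hosting and silently does nothing when joining.
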(event Custom|HostGame
  (CallFunction|CallHostGameImplem))

(event Custom|JoinGame
  (params (ServerIP :type String))
  (CallFunction|CallJoinGameImplem ServerIP))

(event EventBeginPlay)

(event EventTick
  (params (DeltaSeconds :type Float%20%28single-precision%29)))

(fn ConstructionScript)

(fn CallHostGameImplem
  (bind _asmy_game_instance (Utilities|Casting|CastToMyGameInstance (Game|GetGameInstance))
    (:then
      (Default|HostGameImplem _asmy_game_instance))
    (:CastFailed
      (Development|PrintString "Failed Cast"))))

(fn CallJoinGameImplem
  (params (ServerIP :type String))
  (bind _asmy_game_instance (Utilities|Casting|CastToMyGameInstance (Game|GetGameInstance)))
  (Default|JoinGameImplem _asmy_game_instance ServerIP))